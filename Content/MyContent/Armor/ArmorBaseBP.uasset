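; Base armor Blueprint that gives its owner a set of armor mods and relays combat actions to them.
; On BeginPlay, it calls OnConstruction, which adds the stat, two armor and combat style mods to the owner as components and collects them in ArmorModArray.
; OnGrenade and OnMelee forward to every valid mod in that array.
; The grenade and melee damage events are empty.
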(event `self.ReceiveBeginPlay`
  (`self.onConstruction`))

(event `self.onConstruction`
  (bind _returnvalue (`self.GetOwner`))
  (bind _returnvalue_2 (`|AddComponentByClass` _returnvalue (`self.statMod`)))
  (`KismetArrayLibrary.Array_Add` (`self.ArmorModArray`) _returnvalue_2)
  (bind _returnvalue_3 (`|AddComponentByClass` _returnvalue (`self.armorMod1`)))
  (`KismetArrayLibrary.Array_Add` (`self.ArmorModArray`) _returnvalue_3)
  (bind _returnvalue_4 (`|AddComponentByClass` _returnvalue (`self.armorMod2`)))
  (`KismetArrayLibrary.Array_Add` (`self.ArmorModArray`) _returnvalue_4)
  (bind _returnvalue_5 (`|AddComponentByClass` _returnvalue (`self.combatStyleMod`)))
  (`KismetArrayLibrary.Array_Add` (`self.ArmorModArray`) _returnvalue_5))

(event `self.onGrenade`
  (for _array_element (`self.ArmorModArray`)
    (`/Engine/EditorBlueprintResources/StandardMacros.IsValid` _array_element
      (:`Is Valid`
        (`BasePerk.onGrenade` _array_element)))))

(event `self.onMelee`
  (for _array_element (`self.ArmorModArray`)
    (`/Engine/EditorBlueprintResources/StandardMacros.IsValid` _array_element
      (:`Is Valid`
        (`BasePerk.onMelee` _array_element)))))

(event `self.onGrenadeDamage`)

(event `self.onMeleeDamage`)
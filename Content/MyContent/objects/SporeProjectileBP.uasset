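; SporeProjectileBP is a homing projectile that seeks the nearest EnemyCharacter and sets it burning.
; On BeginPlay it launches forward in local space, and FindTarget scans all enemies by distance once to supply the homing component's target.
; Hitting an EnemyCharacter applies a ticking Burn and destroys the projectile, while the Hit event ignores other actors.
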(event `self.ReceiveBeginPlay`
  (bind _projectilemovementcomponent (`self.projectileMovementComponent`))
  (`ProjectileMovementComponent.SetVelocityInLocalSpace` _projectilemovementcomponent (2000.0 0.0 0.0))
  (bind _newparam (`self.FindTarget`))
  (set `ProjectileMovementComponent.HomingTargetComponent` _newparam _projectilemovementcomponent)
  (set `ProjectileMovementComponent.bIsHomingProjectile` true _projectilemovementcomponent))

(event `self.ReceiveHit`
  (params (MyComp :type "PrimitiveComponent Object Reference") (Other :type "Actor Object Reference") (OtherComp :type "PrimitiveComponent Object Reference") (bSelfMoved :type Boolean) (HitLocation :type "Vector Structure") (HitNormal :type "Vector Structure") (NormalImpulse :type "Vector Structure") (Hit :type "HitResult Structure (by ref)"))
  (bind _asenemy_character (cast `/Game/MyContent/Character/enemy/EnemyCharacter` Other))
  (`BaseCharacter.burn` _asenemy_character 5 10)
  (`/Engine/EditorBlueprintResources/StandardMacros.IsValid` self
    (:`Is Valid`
      (`self.K2_DestroyActor`))))

(fn `FindTarget`
  (returns (NewParam :type "SceneComponent Object Reference"))
  (set `self.f_shortestDistance` 10000000.0)
  (bind _outactors (`GameplayStatics.GetAllActorsOfClass` "/Game/MyContent/Character/enemy/EnemyCharacter.EnemyCharacter_C"))
  (for _array_element _outactors
    (bind _returnvalue (`KismetMathLibrary.VSize` (- (`self.K2_GetActorLocation` _array_element) (`self.K2_GetActorLocation`))))
    (if (< _returnvalue (`self.f_shortestDistance`))
      (set `self.f_shortestDistance` _returnvalue)
      (set `self.Target` _array_element)))
  (return (`self.GetComponentByClass` (`self.Target`) "/Script/Engine.SceneComponent")))

(fn `UserConstructionScript`)
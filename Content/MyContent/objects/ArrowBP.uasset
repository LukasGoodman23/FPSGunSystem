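; ArrowBP is the projectile fired by the bow weapon, its owner.
; On BeginPlay it launches forward along its local X axis at the bow's arrow speed.
; On overlap it damages IDamagable actors by the bow's damage value, notifies the bow of BaseCharacter hits, and destroys itself.
; Non-damageable overlaps also destroy it, but a damageable non-character leaves it alive because the failed cast stops execution.
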(event `self.ReceiveActorBeginOverlap`
  (params (OtherActor :type "Actor Object Reference"))
  (if (`KismetSystemLibrary.DoesImplementInterface` OtherActor "/Game/MyContent/Interfaces/iDamagable.iDamagable_C")
    (bind _asbow (cast `/Game/MyContent/guns/baseFiringTypes/bow` (`self.GetOwner`)))
    (message `/Game/MyContent/Interfaces/iDamagable.affect health` OtherActor (`/Game/MyContent/guns/baseFiringTypes/bow.i_arrowAppliedDamage` _asbow) _asbow)
    (bind _asbase_character (cast `BaseCharacter` OtherActor))
    (`GunBase.eventOnHit` _asbow _asbase_character))
  (`self.K2_DestroyActor`))

(event `self.ReceiveBeginPlay`
  (bind _asbow (cast `/Game/MyContent/guns/baseFiringTypes/bow` (`self.GetOwner`)))
  (`ProjectileMovementComponent.SetVelocityInLocalSpace` (`self.projectileMovementComponent`) (`KismetMathLibrary.MakeVector` (`/Game/MyContent/guns/baseFiringTypes/bow.f_arrowSpeed` _asbow))))

(fn `UserConstructionScript`)
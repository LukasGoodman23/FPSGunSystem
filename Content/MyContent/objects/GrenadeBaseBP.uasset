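; Grenade projectile that launches at its owning gun's speed and explodes on hitting a damageable target or after five seconds.
; BeginPlay copies damage, radius and effects from the gun; hits on damageables deal impact damage, while slow hits elsewhere stop movement.
; Explode sphere-overlaps characters for area damage, but truncation flattens the intended outer falloff.
; It destroys itself inside the loop, so only the first character found takes blast damage.
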(event `self.ReceiveHit`
  (params (MyComp :type "PrimitiveComponent Object Reference") (Other :type "Actor Object Reference") (OtherComp :type "PrimitiveComponent Object Reference") (bSelfMoved :type Boolean) (HitLocation :type "Vector Structure") (HitNormal :type "Vector Structure") (NormalImpulse :type "Vector Structure") (Hit :type "HitResult Structure (by ref)"))
  (bind _gun (`self.gun`))
  (if (`KismetSystemLibrary.DoesImplementInterface` Other "/Game/MyContent/Interfaces/iDamagable.iDamagable_C")
    (message `/Game/MyContent/Interfaces/iDamagable.affect health` Other (`self.i_projectileImpactDamage`) _gun (`GunBase.s_damageType` _gun))
    (`self.explode`)
    (elif (< (`KismetMathLibrary.VSize` (`SceneComponent.GetComponentVelocity` (`self.projectileCollision`))) 200.0)
      (`MovementComponent.StopMovementImmediately` (`self.projectileMovementComponent`)))))

(event `self.ReceiveBeginPlay`
  (bind _asgun_base_bp (cast `/Game/MyContent/guns/GunBaseBP` (`self.GetOwner`)))
  (set `self.gun` _asgun_base_bp)
  (`ProjectileMovementComponent.SetVelocityInLocalSpace` (`self.projectileMovementComponent`) (`KismetMathLibrary.MakeVector` (`GunBase.f_nonBulletProjectileSpeed` _asgun_base_bp)))
  (set `self.i_projectileImpactDamage` (`GunBase.i_projectileImpactMaxDamage` _asgun_base_bp))
  (set `self.i_explosionMaxDamage` (`GunBase.i_explosionMaxDamage` _asgun_base_bp))
  (set `self.f_explosionEffectRadius` (`GunBase.f_explosionEffectRadius` _asgun_base_bp))
  (set `self.f_explosionAppearanceScale` (`GunBase.f_explosionAppearanceScale` _asgun_base_bp))
  (set `self.partO_explosionAppearance` (`GunBase.partO_explosionAppearance` _asgun_base_bp))
  (set `self.soundO_explosionSound` (`GunBase.soundO_explosionSound` _asgun_base_bp))
  (`KismetSystemLibrary.K2_SetTimer` null "Explode" 5.0))

(fn `explode`
  (bind _f_explosioneffectradius (`self.f_explosionEffectRadius`))
  (bind _i_explosionmaxdamage (`self.i_explosionMaxDamage`))
  (bind _returnvalue (`SceneComponent.K2_GetComponentLocation` (`self.projectileCollision`)))
  (`/Engine/EditorBlueprintResources/StandardMacros.IsValid` self
    (:`Is Valid`
      (`GameplayStatics.SpawnEmitterAtLocation` (`self.partO_explosionAppearance`) _returnvalue (struct) (`KismetMathLibrary.Conv_DoubleToVector` (`self.f_explosionAppearanceScale`)))
      (`GameplayStatics.PlaySoundAtLocation` (`self.soundO_explosionSound`) _returnvalue (struct) 1.0 1.0 0.0 null null null)
      (bind (_outactors _returnvalue_2) (`KismetSystemLibrary.SphereOverlapActors` _returnvalue (`self.f_explosionEffectRadius`) (`self.Object Types`) "/Script/FPSGunSystem.BaseCharacter"))
      (if _returnvalue_2
        (for _array_element _outactors
          (`/Engine/EditorBlueprintResources/StandardMacros.IsValid` self
            (:`Is Valid`
              (bind _returnvalue_location (`KismetMathLibrary.BreakTransform` (`self.GetTransform` _array_element)))
              (bind _returnvalue_3 (`KismetMathLibrary.VSize` (- _returnvalue _returnvalue_location)))
              (if (< _returnvalue_3 (/ _f_explosioneffectradius 2.0))
                (message `/Game/MyContent/Interfaces/iDamagable.affect health` _array_element _i_explosionmaxdamage null "")
                (else
                  (message `/Game/MyContent/Interfaces/iDamagable.affect health` _array_element (* _i_explosionmaxdamage (- 1 (`KismetMathLibrary.FTrunc` (/ _returnvalue_3 _f_explosioneffectradius)))) null "")))
              (`/Engine/EditorBlueprintResources/StandardMacros.IsValid` self :!label _label
                (:`Is Valid`
                  (`self.K2_DestroyActor`))))))
        (else
          (goto _label))))))

(fn `UserConstructionScript`)
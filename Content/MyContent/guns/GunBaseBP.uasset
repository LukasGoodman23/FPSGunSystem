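; Base first-person gun, handling firing, aim-down-sights, kickback, melee and grenade-throw animation, with five perk components notified of gun events.
; Shoot applies stats, bends aim toward characters using tracer traces, then fires once per spread-cone wedge.
; Hitscan shots apply falloff and headshot damage within one frame of bullet travel, otherwise spawning a bullet actor; non-hitscan guns spawn projectiles.
; Timelines drive arm-joint rotations, ADS zoom and melee capsule-trace damage.
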(event `startShooting`
  (set `self.b_isFiring` true))

(event `self.ReceiveTick`
  (params (DeltaSeconds :type "Float (single-precision)"))
  (if (`self.b_isAltFire`)
    (bind _asfirst_person_character (cast `/Game/FirstPersonBP/Blueprints/FirstPersonCharacter` (`GameplayStatics.GetPlayerCharacter` 0)))
    (`SceneComponent.K2_SetWorldRotation` (`/Game/FirstPersonBP/Blueprints/FirstPersonCharacter.FirstPersonCamera` _asfirst_person_character) (`Controller.GetControlRotation` (`GameplayStatics.GetPlayerController` 0)) false false) ; Allow ADS Up and Down Rotation
  ))

(event `stopShooting`
  (set `self.b_isFiring` false)
  (`TimelineComponent.PlayFromStart` (`self.resetKickback`)))

(event `startAltFire`
  (bind _aimdownsights (`self.aimDownSights`))
  (bind _adszoom (`self.adsZoom`))
  (bind _returnvalue (/ 1.0 (`self.f_appliedADSTime`)))
  (set `self.b_isAltFire` true)
  (for _array_element (`self.Perk Array`)
    (bind _asbase_perk_bp (cast `/Game/MyContent/Perks/BasePerkBP` _array_element))
    (`/Game/MyContent/Perks/BasePerkBP.stopAimDownSights` _asbase_perk_bp))
  (`TimelineComponent.SetPlayRate` _aimdownsights _returnvalue)
  (`TimelineComponent.Play` _aimdownsights)
  (`TimelineComponent.SetPlayRate` _adszoom _returnvalue)
  (`TimelineComponent.Play` _adszoom))

(event `stopAltFire`
  (bind _aimdownsights (`self.aimDownSights`))
  (bind _adszoom (`self.adsZoom`))
  (bind _returnvalue (/ 1.0 (`self.f_appliedADSTime`)))
  (set `self.b_isAltFire` false)
  (for _array_element (`self.Perk Array`)
    (bind _asbase_perk_bp (cast `/Game/MyContent/Perks/BasePerkBP` _array_element))
    (`/Game/MyContent/Perks/BasePerkBP.stopAimDownSights` _asbase_perk_bp))
  (`TimelineComponent.SetPlayRate` _aimdownsights _returnvalue)
  (`TimelineComponent.Reverse` _aimdownsights)
  (`TimelineComponent.SetPlayRate` _adszoom _returnvalue)
  (`TimelineComponent.Reverse` _adszoom))

(event `InputAction|Reload`
  (params (Key :type "Key Structure")))

(event `holdReload`)

(event `/Game/MyContent/Interfaces/iKilled.youKilledMe`
  (for _array_element (`self.Perk Array`)
    (bind _asbase_perk_bp (cast `/Game/MyContent/Perks/BasePerkBP` _array_element))
    (`/Game/MyContent/Perks/BasePerkBP.onKill` _asbase_perk_bp)))

(event `melee`
  (`TimelineComponent.PlayFromStart` (`self.warlockMelee`)))

(event `Grenade`
  (`KismetSystemLibrary.PrintString` "Grenade")
  (`TimelineComponent.PlayFromStart` (`self.ThrowGrenade`)))

(event `self.fire`
  (bind _i_currentammocount (`self.i_currentAmmoCount`))
  (bind _s_damagetype (`self.s_damageType`))
  (if (`self.b_isHitscan`)
    ;[1 1 1] Hitscan Hipfire
    (bind _asfirst_person_character (cast `/Game/FirstPersonBP/Blueprints/FirstPersonCharacter` (`self.GetParentActor`)))
    (if (> _i_currentammocount 0)
      (`/Engine/EditorBlueprintResources/StandardMacros.DecrementInt` _i_currentammocount
        (:`  `
          (bind _shootlocation (`/Game/FirstPersonBP/Blueprints/FirstPersonCharacter.ShootLocation` _asfirst_person_character))
          (bind _returnvalue (`SceneComponent.K2_GetComponentLocation` _shootlocation))
          (bind _outhit (`KismetSystemLibrary.LineTraceSingleForObjects` _returnvalue (+ (* (`KismetMathLibrary.GetForwardVector` (`SceneComponent.K2_GetComponentRotation` _shootlocation)) (`self.f_maxBulletDistance`)) _returnvalue) (`self.Object Types`) false (`|MakeArray` (`self.GetParentActor`)) "ForDuration"))
          (bind (_bblockinghit _binitialoverlap _time _distance _location _impactpoint _normal _impactnormal _physmat _hitactor _hitcomponent _hitbonename) (`GameplayStatics.BreakHitResult` _outhit))
          (set `self.f_shotDistance` _distance)
          (bind _output_get (set `self.s_hitBoneName` (`KismetStringLibrary.Conv_NameToString` _hitbonename)))
          (`GameplayStatics.PlaySoundAtLocation` (`self.soundO_firingSound`) (`SceneComponent.K2_GetComponentLocation` (`self.BarrelReferencePoint`)) (struct) 1.0 1.0 0.0 null null null)
          (bind _returnvalue_2 (`GameplayStatics.SpawnEmitterAttached` (`self.particleO_muzzleFlash`) (`self.BarrelReferencePoint`) "None" (0.0 0.0 0.0) (struct :`Yaw` 90.0) (`self.FlashScale`)))
          (message `AnimationDataController.SetPlayLength` _returnvalue_2 0.01 true)
          (if (< _distance (/ (`self.f_BulletSpeed`) 60.0))
            (if _bblockinghit
              (bind _returnvalue_3 (`ActorComponent.GetOwner` _hitcomponent))
              (bind _asbase_character (cast `BaseCharacter` _returnvalue_3))
              (`/Engine/EditorBlueprintResources/StandardMacros.IsValid` _asbase_character
                (:`Is Valid`
                  (if (`KismetSystemLibrary.DoesImplementInterface` _returnvalue_3 "/Game/MyContent/Interfaces/iDamagable.iDamagable_C")
                    (`self.calculateDamageFalloff`)
                    (`self.onHit` _asbase_character)
                    (if (== (`self.s_hitBoneName`) "Head")
                      (message `/Game/MyContent/Interfaces/iDamagable.affect health` _asbase_character (`KismetMathLibrary.FTrunc` (* (`self.f_headshotMultiplier`) (`self.i_appliedDamage`))) self _s_damagetype)
                      (for _array_element (`self.Perk Array`)
                        (bind _asbase_perk_bp (cast `/Game/MyContent/Perks/BasePerkBP` _array_element))
                        (`/Game/MyContent/Perks/BasePerkBP.onPrecisionHit` _asbase_perk_bp))
                      (else
                        (message `/Game/MyContent/Interfaces/iDamagable.affect health` _asbase_character (`self.i_appliedDamage`) self _s_damagetype)))))))
            (else
              (`self.calculateDamageFalloff`)
              (`|SpawnActorFromClass` "/Game/MyContent/objects/BulletBP.BulletBP_C" (`SceneComponent.K2_GetComponentToWorld` _shootlocation) "Undefined" "OverrideRootScale" self null) ; Shoot Bullet Actor
            )))))
    (else
      ;[1 1 1] Projectile Hipfire
      (bind _asfirst_person_character_2 (cast `/Game/FirstPersonBP/Blueprints/FirstPersonCharacter` (`self.GetParentActor`)))
      (if (> (`self.i_currentAmmoCount`) 0)
        (bind _output_get_2 (set `self.r_rotationStorage` (`SceneComponent.K2_GetComponentRotation` (`/Game/FirstPersonBP/Blueprints/FirstPersonCharacter.FirstPersonCamera` _asfirst_person_character_2))))
        (`/Engine/EditorBlueprintResources/StandardMacros.DecrementInt` (`self.i_currentAmmoCount`)
          (:`  `
            (bind _returnvalue_4 (`|SpawnActorFromClass` (`self.projectile`) (`KismetMathLibrary.MakeTransform` (`SceneComponent.K2_GetComponentLocation` (`/Game/FirstPersonBP/Blueprints/FirstPersonCharacter.ShootLocation` _asfirst_person_character_2)) _output_get_2) "Undefined" "OverrideRootScale" self null))
            (set `self.projectileO_activeProjectile` _returnvalue_4)
            (`self.recoil`)
            (`GameplayStatics.PlaySoundAtLocation` (`self.soundO_firingSound`) (`SceneComponent.K2_GetComponentLocation` (`self.BarrelReferencePoint`)) (struct) 1.0 1.0 0.0 null null null)
            (`GameplayStatics.SpawnEmitterAttached` (`self.particleO_muzzleFlash`) (`self.BarrelReferencePoint`) "None" (0.0 0.0 0.0) (struct :`Yaw` 90.0) (0.03 0.03 0.03))))))))

(event `self.ReceiveBeginPlay`
  (bind _returnvalue (`|AddComponentByClass` (`self.mod`)))
  (`KismetArrayLibrary.Array_Add` (`self.Perk Array`) _returnvalue)
  (bind _returnvalue_2 (`|AddComponentByClass` (`self.barrelPerk`)))
  (`KismetArrayLibrary.Array_Add` (`self.Perk Array`) _returnvalue_2)
  (bind _returnvalue_3 (`|AddComponentByClass` (`self.magazinePerk`)))
  (`KismetArrayLibrary.Array_Add` (`self.Perk Array`) _returnvalue_3)
  (bind _returnvalue_4 (`|AddComponentByClass` (`self.trait1`)))
  (`KismetArrayLibrary.Array_Add` (`self.Perk Array`) _returnvalue_4)
  (bind _returnvalue_5 (`|AddComponentByClass` (`self.trait2`)))
  (`KismetArrayLibrary.Array_Add` (`self.Perk Array`) _returnvalue_5)
  (`KismetSystemLibrary.Delay` 0.1)
  (set `self.b_usedBefore` true))

(fn `aimAssist`
  (locals (endPointMultiplier :type "Vector Structure" :default (100000.0 100000.0 100000.0)) (shotDistanceMultiplier :type "Float (double-precision)" :default 100000.0))
  (bind _asfirst_person_character (cast `/Game/FirstPersonBP/Blueprints/FirstPersonCharacter` (`self.GetParentActor`)))
  (`self.defineOnGroundRadius` (`self.f_currentAimAssistConeAngle`)) ; Set the radius of the aim assist cone
  (bind _shootlocation (`/Game/FirstPersonBP/Blueprints/FirstPersonCharacter.ShootLocation` _asfirst_person_character))
  (`SceneComponent.K2_AddRelativeRotation` _shootlocation (`self.r_shotDirectionRotator`) false false) ; Rotate Tracer Vector
  (bind _returnvalue (`SceneComponent.K2_GetComponentLocation` _shootlocation))
  (bind _outhit (`KismetSystemLibrary.LineTraceSingleForObjects` _returnvalue (+ (* (`KismetMathLibrary.GetForwardVector` (`SceneComponent.K2_GetComponentRotation` _shootlocation)) (`local.shotDistanceMultiplier`)) _returnvalue) (`self.Object Types`) false (`|MakeArray` (`self.GetParentActor`)))) ; Fire Tracer to Test for a Hit on a BaseCharacter
  (cast `BaseCharacter` (`.HitActor` (`GameplayStatics.BreakHitResult` _outhit)) ; Test if Hit Actor is a BaseCharacter
    (:`CastFailed`
      (`SceneComponent.K2_SetRelativeRotation` :`self` _shootlocation) ; Reset Firing Rotator
      (for _ (range (`self.i_numberOfAimAssitTracerShots`))
        (`self.setCartesianCoordinates` 0 0.0 (`self.f_insideConeRadius`)) ; Set the Cartesian Coordinates of the Point in the Circle Cross Section of the Firing Cone at the Projection Distance
        (`self.setFiringRotator`) ; Set the Rotator using the Cartesian Coordinates
        (`SceneComponent.K2_AddRelativeRotation` _shootlocation (`self.r_shotDirectionRotator`) false false) ; Rotate Tracer Vector
        (bind _returnvalue_2 (`SceneComponent.K2_GetComponentLocation` _shootlocation))
        (bind _outhit_2 (`KismetSystemLibrary.LineTraceSingleForObjects` _returnvalue_2 (+ (* (`KismetMathLibrary.GetForwardVector` (`SceneComponent.K2_GetComponentRotation` _shootlocation)) (`local.shotDistanceMultiplier`)) _returnvalue_2) (`self.Object Types`) false (`|MakeArray` (`self.GetParentActor`)))) ; Fire Tracer to Test for a Hit on a BaseCharacter
        (cast `BaseCharacter` (`.HitActor` (`GameplayStatics.BreakHitResult` _outhit_2)) ; Test if Hit Actor is a BaseCharacter
          (:`then`
            (break))
          (:`CastFailed`
            (`SceneComponent.K2_SetRelativeRotation` :`self` _shootlocation) ; Reset Firing Rotator
          ))))))

(fn `getFiringConeRadius`
  (locals (I_CurrentWedgeIndex :type Integer))
  (bind _b_isaltfire (`self.b_isAltFire`))
  (bind _asfirst_person_character (cast `/Game/FirstPersonBP/Blueprints/FirstPersonCharacter` (`self.GetParentActor`)))
  (if (`NavMovementComponent.IsFalling` (`Character.CharacterMovement` _asfirst_person_character))
    (if _b_isaltfire
      (`self.defineInAirRadius` (`self.f_currentTotalADSConeAngle`))
      (else
        (`self.defineInAirRadius` (`self.f_currentTotalConeAngle`))))
    (elif _b_isaltfire
      (`self.defineOnGroundRadius` (`self.f_currentTotalADSConeAngle`))
      (else
        (`self.defineOnGroundRadius` (`self.f_currentTotalConeAngle`))))))

(fn `recoil`)

(fn `shoot`
  (set `self.i_appliedDamage` (`self.i_baseDamage`))
  (`self.applyStats`) ; Apply Range and Impact Stats
  (for _array_element (`self.Perk Array`)
    (bind _asbase_perk_bp (cast `/Game/MyContent/Perks/BasePerkBP` _array_element))
    (`/Game/MyContent/Perks/BasePerkBP.gunShoot` _asbase_perk_bp))
  (`self.aimAssist`) ; Rotate Firing Cone using Aim Assist Cone
  (`self.getFiringConeRadius`) ; Set the Firing Cone Radius at the Projection Distance
  (bind _asfirst_person_character (cast `/Game/FirstPersonBP/Blueprints/FirstPersonCharacter` (`self.GetParentActor`)))
  (for _index (range (`self.i_NumberOfInsideAimWedges`))
    (`self.setCartesianCoordinates` _index 0.0 (`self.f_insideConeRadius`)) ; Set the Cartesian Coordinates of the Point in the Circle Cross Section of the Firing Cone at the Projection Distance
    (`self.setFiringRotator`) ; Set the Rotator using the Cartesian Coordinates
    (bind _shootlocation (`/Game/FirstPersonBP/Blueprints/FirstPersonCharacter.ShootLocation` _asfirst_person_character))
    (`SceneComponent.K2_AddRelativeRotation` _shootlocation (`self.r_shotDirectionRotator`) false false)
    (`self.fire`)
    ;[1 1 1] Reset Firing Rotator
    (`SceneComponent.K2_SetRelativeRotation` :`self` _shootlocation)
    (`/Engine/EditorBlueprintResources/StandardMacros.IncrementInt` (`self.i_currentAmmoCount`)
      (:`  `
        (`TimelineComponent.PlayFromStart` (`self.kickBack`)))))
  (`/Engine/EditorBlueprintResources/StandardMacros.DecrementInt` (`self.i_currentAmmoCount`)))

(fn `UserConstructionScript`
  (`SceneComponent.K2_AttachToComponent` (`self.Gun`) (`self.Arms`) "GripPoint" "KeepRelative" "KeepRelative" "KeepRelative" true))

(fn `yawPitchInput`
  (params (Character :type "/Game/FirstPersonBP/Blueprints/FirstPersonCharacter Object Reference") (Pitch :type "Float (double-precision)") (Yaw :type "Float (double-precision)")))